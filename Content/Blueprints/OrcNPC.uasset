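; Orc quest-giver NPC that shows a quest mark and lets the Hunter know when it is in interaction range.
; Capsule overlaps set or clear the Hunter's NPC reference and, when a quest is available or claimable, toggle the advice prompt on the UI widget found by class.
; Tick rotates the quest mark widget toward the player character, while UpdateQuestState forwards the claimable state to its QuestMarks widget.
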(event `self.ReceiveTick`
  (params (DeltaSeconds :type "Float (single-precision)"))
  (bind _widget (`self.Widget`))
  ;[1 0.2671 0] The quest mark is always oriented to the character
  (`SceneComponent.K2_SetWorldRotation` _widget (`KismetMathLibrary.FindLookAtRotation` (`SceneComponent.K2_GetComponentLocation` _widget) (`self.K2_GetActorLocation` (`GameplayStatics.GetPlayerCharacter` 0))) false false))

(event `self.Capsule.OnComponentBeginOverlap`
  (params (OverlappedComponent :type "PrimitiveComponent Object Reference") (OtherActor :type "Actor Object Reference") (OtherComp :type "PrimitiveComponent Object Reference") (OtherBodyIndex :type Integer) (bFromSweep :type Boolean) (SweepResult :type "HitResult Structure (by ref)"))
  ;[0.7373 0.298 0.3373] Interact collision events
  (bind _ashunter (cast `/Game/Blueprints/Hunter` OtherActor))
  (set `/Game/Blueprints/Hunter.NPC` self _ashunter)
  (if (or (`self.QuestAvailable?`) (`self.ClaimableQuest?`))
    (bind _foundwidgets (`WidgetBlueprintLibrary.GetAllWidgetsOfClass` "/Game/Blueprints/Widgets/UI.UI_C"))
    (`/Game/Blueprints/Widgets/UI.ShowAdvice` (`|GetArrayItem` _foundwidgets) true)))

(event `self.Capsule.OnComponentEndOverlap`
  (params (OverlappedComponent :type "PrimitiveComponent Object Reference") (OtherActor :type "Actor Object Reference") (OtherComp :type "PrimitiveComponent Object Reference") (OtherBodyIndex :type Integer))
  ;[0.7373 0.298 0.3373] Interact collision events
  (bind _ashunter (cast `/Game/Blueprints/Hunter` OtherActor))
  (set `/Game/Blueprints/Hunter.NPC` null _ashunter)
  (if (or (`self.QuestAvailable?`) (`self.ClaimableQuest?`))
    (bind _foundwidgets (`WidgetBlueprintLibrary.GetAllWidgetsOfClass` "/Game/Blueprints/Widgets/UI.UI_C"))
    (`/Game/Blueprints/Widgets/UI.ShowAdvice` (`|GetArrayItem` _foundwidgets) false)))

(event `UpdateQuestState`
  (params (`Claimable?` :type Boolean))
  ;[1 1 0] Updates the UI of the quest marks
  (`/Game/Blueprints/Widgets/QuestMarks.QuestUpdate` (cast `/Game/Blueprints/Widgets/QuestMarks` (`WidgetComponent.GetWidget` (`self.Widget`)) :!pure true) `Claimable?`))

(fn `UserConstructionScript`)