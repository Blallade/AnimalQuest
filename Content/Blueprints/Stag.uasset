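; Stag is a prey animal character that flees the Hunter by speeding up when it detects one, and can die.
; A vision overlap volume or any AI perception update sets near and seen flags and raises walk speed.
; Losing sight, and also every perception update, starts a delay that restores slow walking unless re-spotted.
; Death runs once, disabling movement, playing sound and blood, then printing a placeholder mission-count message.
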(event `self.VisionRadious.OnComponentBeginOverlap`
  (params (OverlappedComponent :type "PrimitiveComponent Object Reference") (OtherActor :type "Actor Object Reference") (OtherComp :type "PrimitiveComponent Object Reference") (OtherBodyIndex :type Integer) (bFromSweep :type Boolean) (SweepResult :type "HitResult Structure (by ref)"))
  ;[1 0.07059 0.07059] Stag sees hunter events
  (cast `/Game/Blueprints/Hunter` OtherActor)
  (set `self.HunterNear?` true :!label _label)
  (set `self.HunterSeen?` true)
  (set `CharacterMovementComponent.MaxWalkSpeed` 600.0 (`self.CharacterMovement`)))

(event `self.AIPerception.OnPerceptionUpdated`
  (params (UpdatedActors :type "Array of Actor Object Reference (by ref)"))
  ;[0.5272 0.114 1] Stag hears hunter
  ;[1 0.07059 0.07059] Stag sees hunter events
  (`|ExecutionSequence`
    (:`then_0`
      (goto _label))
    (:`then_1`
      (set `self.HunterSeen?` false :!label _label_2)
      (`KismetSystemLibrary.Delay` 5.0)
      (if (not (`self.HunterSeen?`))
        (set `self.HunterNear?` false)
        (set `CharacterMovementComponent.MaxWalkSpeed` 150.0 (`self.CharacterMovement`))))))

(event `self.VisionRadious.OnComponentEndOverlap`
  (params (OverlappedComponent :type "PrimitiveComponent Object Reference") (OtherActor :type "Actor Object Reference") (OtherComp :type "PrimitiveComponent Object Reference") (OtherBodyIndex :type Integer))
  ;[1 0.07059 0.07059] Stag sees hunter events
  (cast `/Game/Blueprints/Hunter` OtherActor)
  (goto _label_2))

(event `Death`
  ;[0.1562 0 0] Death event
  (`/Engine/EditorBlueprintResources/StandardMacros.DoOnce` false
    (:`Completed`
      (`CharacterMovementComponent.DisableMovement` (`self.CharacterMovement`))
      (set `self.Dead?` true)
      (`GameplayStatics.SpawnSound2D` null 1.0 1.0 0.0 null)
      (bind _returnvalue (`GameplayStatics.SpawnEmitterAttached` "/Game/Particles/P_Blood.P_Blood" (`self.Mesh`) "None" (0.0 0.0 100.0)))
      (`KismetSystemLibrary.Delay` 1.0)
      (`ParticleSystemComponent.EndTrails` _returnvalue)
      (bind _foundwidgets (`WidgetBlueprintLibrary.GetAllWidgetsOfClass` null))
      (`KismetSystemLibrary.PrintString` "Contabiliza +1 a la misión"))))

(fn `UserConstructionScript`)